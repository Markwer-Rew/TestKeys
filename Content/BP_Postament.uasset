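; BP_Postament is an interactable pedestal that takes the player's carried key and opens the level's BP_Door, found on BeginPlay.
; Interact works once, only while the player is grabbing: it opens the door and plays a Timeline that scales up the placed Item.
; The Timeline update also clears the player's held mesh, grab state and Focused flag.
; Focus sets the name widget to an interact prompt, a no-key message or blank.
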(event `self.ReceiveBeginPlay`
  (`parent.ReceiveBeginPlay`)
  (bind _returnvalue (`GameplayStatics.GetActorOfClass` "/Game/BP_Door.BP_Door_C"))
  (set `self.Door` _returnvalue))

(event `/Game/BPI_Interact.Interact`
  (if (`/Game/FirstPerson/Blueprints/BP_FirstPersonCharacter.IsGrabbed` (`self.As BP First Person Character`))
    (`/Engine/EditorBlueprintResources/StandardMacros.DoOnce` false
      (:`Completed`
        (`/Game/BP_Door.Open` (`self.Door`))
        (bind (_direction _move) (`Timeline|Timeline`)
          (:`Update`
            (`SceneComponent.SetWorldScale3D` (`self.Item`) (`KismetMathLibrary.Conv_DoubleToVector` (`KismetMathLibrary.Lerp` 0.0 0.15 _move)))
            (`StaticMeshComponent.SetStaticMesh` (`/Game/FirstPerson/Blueprints/BP_FirstPersonCharacter.EquipItem` (`self.As BP First Person Character`)) null)
            (bind _output_get (set `/Game/FirstPerson/Blueprints/BP_FirstPersonCharacter.IsGrabbed` false (`self.As BP First Person Character`)))
            (set `self.Focused` _output_get)))))))

(event `/Game/BPI_Interact.Focus`
  (params (Enable :type Boolean))
  (if (`self.Focused`)
    (if (`/Game/FirstPerson/Blueprints/BP_FirstPersonCharacter.IsGrabbed` (`self.As BP First Person Character`))
      (bind _output_get (set `self.Item Name` "Press E to interact"))
      (`TextBlock.SetText` (`/Game/WBP_FocusName.TextName` (`self.As WBP Focus Name`)) _output_get)
      (`SceneComponent.SetVisibility` (`self.Name`) Enable false)
      (else
        (bind _output_get_2 (set `self.Item Name` "You Have no Key"))
        (`TextBlock.SetText` (`/Game/WBP_FocusName.TextName` (`self.As WBP Focus Name`)) _output_get_2)
        (`SceneComponent.SetVisibility` (`self.Name`) Enable false)))
    (else
      (bind _output_get_3 (set `self.Item Name` ""))
      (`TextBlock.SetText` (`/Game/WBP_FocusName.TextName` (`self.As WBP Focus Name`)) _output_get_3)
      (`SceneComponent.SetVisibility` (`self.Name`) Enable false))))

(fn `UserConstructionScript`
  (`parent.UserConstructionScript`))