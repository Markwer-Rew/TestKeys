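; Door Blueprint that swings open once it has received enough matching Open calls.
; The Open event compares indices, increments a Points counter on a match, and plays the OpenDoor timeline when Points reaches NeedKeys.
; The timeline drives a yaw lerp on the relative rotation of the Point component, swinging it to roughly a right angle.
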(event `Open`
  (params (Index :type Integer))
  (if (== Index (`self.Index`))
    (`/Engine/EditorBlueprintResources/StandardMacros.IncrementFloat` (`self.Points`)
      (:`  `
        (if (>= (`self.Points`) (`self.NeedKeys`))
          (bind (_direction _newtrack_0) (`Timeline|OpenDoor`)
            (:`Update`
              (`SceneComponent.K2_SetRelativeRotation` (`self.Point`) (`KismetMathLibrary.MakeRotator` 0.0 0.0 (`KismetMathLibrary.Lerp` 0.0 -95.0 _newtrack_0)) false false))))))))

(fn `UserConstructionScript`)