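; BP_InteractItem is an interactable world item that shows a name label when focused and is destroyed when interacted with.
; On BeginPlay it casts the Name widget component's widget to WBP_FocusName and sets its text to ItemName.
; The Focus event toggles the label's visibility, and the Interact event destroys the actor.
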(event `self.ReceiveBeginPlay`
  (bind _aswbp_focus_name (cast `/Game/WBP_FocusName` (`WidgetComponent.GetWidget` (`self.Name`))))
  (set `self.As WBP Focus Name` _aswbp_focus_name)
  (`TextBlock.SetText` (`/Game/WBP_FocusName.TextName` (`self.As WBP Focus Name`)) (`self.Item Name`)))

(event `/Game/BPI_Interact.Interact`
  (`self.K2_DestroyActor`))

(event `/Game/BPI_Interact.Focus`
  (params (Enable :type Boolean))
  (`SceneComponent.SetVisibility` (`self.Name`) Enable false))

(fn `UserConstructionScript`)